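; Test actor that exercises Enhanced Input and an additive oscillation function, showing results through debug prints.
; BeginPlay adds the IMC_Test mapping context to player 0, and the IA_Test action resets Timer and prints a greeting.
; Each Tick feeds Timer and delta time into OscillateAdditive, adds the result to Accum and prints the running total.
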(event `self.ReceiveBeginPlay`
  (`EnhancedInputSubsystemInterface.AddMappingContext` (pcsubsystem `EnhancedInputLocalPlayerSubsystem` (`GameplayStatics.GetPlayerController` 0)) "/Game/IMC_Test.IMC_Test" 0 (struct)))

(event `EnhancedInput|/Game/IA_Test`
  (params (ActionValue :type Boolean) (ElapsedSeconds :type "Float (double-precision)") (TriggeredSeconds :type "Float (double-precision)") (InputAction :type "InputAction Object Reference" :default "/Game/IA_Test.IA_Test"))
  (:`Triggered`
    (set `self.Timer` 0.0)
    (`KismetSystemLibrary.PrintString` "Hello")))

(event `self.ReceiveTick`
  (params (DeltaSeconds :type "Float (single-precision)"))
  (bind _returnvalue (`GameplayStaticsExtended.OscillateAdditive` (`self.Timer`) 5.0 DeltaSeconds 5.0))
  (bind _output_get (set `self.Accum` (+ _returnvalue (`self.Accum`))))
  (`KismetSystemLibrary.PrintString` (`KismetStringLibrary.Conv_DoubleToString` _output_get)))

(fn `UserConstructionScript`)